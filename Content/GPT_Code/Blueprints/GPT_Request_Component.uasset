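; GPT request component that sends a chat history to OpenAI's text-davinci-003 completion model and returns the reply.
; RequestResponse builds an inline Python script from the API key, history and token limit, then runs it through ExecutePythonCommandEx.
; It string-splits the logged output to extract the "text" field, strips newlines and returns it with a validity flag, optionally printing debug output.
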(event EventBeginPlay)

(event EventTick
  (params (DeltaSeconds :type Float%20%28single-precision%29)))

(fn RequestResponse
  (params (Chat%20History :type String))
  (bind _debug (Variables|Default|GetDebug))
  (bind (_commandresult _logoutput _returnvalue) (Class|PythonScriptLibrary|ExecutePythonCommandEx (Utilities|String|Append (Utilities|String|Append "import openai 
openai.api_key = \"" (Variables|Default|GetOpenAIKey) "\" 
prompt = \"") (Utilities|String|Replace Chat%20History " 
" "\\n") "\" 
response = openai.Completion.create(engine=\"text-davinci-003\", prompt=prompt, max_tokens=" (Utilities|String|ToString(Integer) (Variables|Default|GetMaxToken)) ") 
print(response)")))
  (if (Utilities|Array|IsEmpty _logoutput)
    (return "" false)
    (else
      (if _debug
        (Development|PrintString (Utilities|String|Append "Reponse: " (Utilities|String|ToString(Boolean) _debug) " 
" _commandresult)))
      (return (Utilities|String|Replace (.LeftS (Utilities|String|Split (.RightS (Utilities|String|Split (.output (Utilities|Array|Get(acopy) _logoutput)) "\"text\": \"")) "\"")) "\\n" " 
") _returnvalue))))