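; DefaultMacro is a set of Blueprint helpers that flatten stats, surroundings and available actions into plain strings.
; The stats helper walks the map keys and writes each value as a truncated score out of 100.
; The surroundings helper concatenates its entries without separators.
; The action helper iterates the whole Actions enum into a comma-prefixed list, so it applies no filtering by game state.
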(fn ConvertStatstoText
  (params (Stats :type Map%20of%20Strings%20to%20Reals))
  (bind _keys (Utilities|Map|Keys Stats))
  (for _array_element _keys
    (LocalVariables|SetTempString (Utilities|String|Append (LocalVariables|GetTempString) " 
" _array_element ":" (Utilities|String|ToString(Integer) (Math|Float|Truncate (* (.Value (Utilities|Map|Find Stats _array_element)) 1e+02))) "/100")))
  (return (LocalVariables|GetTempString)))

(fn SurroundingInfotoText
  (params (Surrounding%20info :type Array%20of%20Strings))
  (for _array_element Surrounding%20info
    (LocalVariables|SetTempString (Utilities|String|Append (LocalVariables|GetTempString) " 
" _array_element)))
  (return (LocalVariables|GetTempString)))

(fn PossibleAction
  (bind _enumvalue (|ForEachActionsEnum)
    (:LoopBody
      (LocalVariables|SetTempString (Utilities|String|Append (LocalVariables|GetTempString) "," (Utilities|String|EnumtoString _enumvalue))))
    (:then
      (return (LocalVariables|GetTempString)))))