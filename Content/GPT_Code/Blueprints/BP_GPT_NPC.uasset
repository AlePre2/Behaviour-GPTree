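; GPT-driven NPC that opens a chat UI when the player overlaps it and can run an optional GPT behaviour tree.
; BeginPlay seeds chat history from name and info, then activates the tree if enabled.
; View box overlaps write enemy visibility into the tree's surrounding info and toggle an icon.
; An Action event executes the given action: moving, raising a stat for eating or drinking, or spawning attack and victory effects.
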(event OnComponentBeginOverlap(InteractionCollision)
  (params (OverlappedComponent :type Primitive%20Component%20Object%20Reference) (OtherActor :type Actor%20Object%20Reference) (OtherComp :type Primitive%20Component%20Object%20Reference) (OtherBodyIndex :type Integer) (bFromSweep :type Boolean) (SweepResult :type Hit%20Result%20Structure%20%28by%20ref%29))
  (bind _returnvalue (Game|GetPlayerController 0))
  (if (Variables|GPT|GetCanChat)
    (if (== (Game|Player|GetPlayerPawn 0) OtherActor)
      (bind _returnvalue_2 (UserInterface|CreateWidget "/Game/GPT_Code/UI/NPC_UI.NPC_UI_C" 0 self (Variables|GPT|GetFirstInteraction)))
      (UserInterface|Viewport|AddtoViewport _returnvalue_2 0)
      (Input|SetInputModeUIOnly _returnvalue _returnvalue_2 "DoNotLock")
      (Input|DisableInput (Game|Player|GetPlayerPawn 0) _returnvalue)
      (Variables|/Script/Engine.PlayerController|SetbShowMouseCursor _returnvalue true)
      (Variables|GPT|SetFirstInteraction false))))

(event OnComponentBeginOverlap(ViewBox)
  (params (OverlappedComponent :type Primitive%20Component%20Object%20Reference) (OtherActor :type Actor%20Object%20Reference) (OtherComp :type Primitive%20Component%20Object%20Reference) (OtherBodyIndex :type Integer) (bFromSweep :type Boolean) (SweepResult :type Hit%20Result%20Structure%20%28by%20ref%29))
  (if (== (Game|Player|GetPlayerPawn 0) OtherActor)
    (Variables|Default|SetPlayerInVisual true)
    (Utilities|Array|SetArrayElem (Variables|/Game/GPT_Code/Blueprints/GPT_BehaviourTree.GPT_BehaviourTree_C|GetSurroundingInfo (Variables|Default|GetGPT_BehaviourTree)) 0 "You can see the enemy" true)
    (Rendering|SetVisibility (Variables|Default|GetPlayerFoundIcon) true false)))

(event OnComponentEndOverlap(ViewBox)
  (params (OverlappedComponent :type Primitive%20Component%20Object%20Reference) (OtherActor :type Actor%20Object%20Reference) (OtherComp :type Primitive%20Component%20Object%20Reference) (OtherBodyIndex :type Integer))
  (if (== (Game|Player|GetPlayerPawn 0) OtherActor)
    (Variables|Default|SetPlayerInVisual false)
    (Utilities|Array|SetArrayElem (Variables|/Game/GPT_Code/Blueprints/GPT_BehaviourTree.GPT_BehaviourTree_C|GetSurroundingInfo (Variables|Default|GetGPT_BehaviourTree)) 0 "You do not see the enemy" true)
    (Rendering|SetVisibility (Variables|Default|GetPlayerFoundIcon) false false)))

(event EventBeginPlay
  (Variables|GPT|SetChatHistory (Utilities|String|Append "" (Variables|GPT|GetNPC%20Infos) " 
" (Utilities|String|Append (Variables|GPT|GetNPC%20Name) ":")))
  (if (Variables|GPT|GetBehaviourTreeActivated)
    (Default|ComponentActivated (Variables|Default|GetGPT_BehaviourTree))))

(event EventAction
  (params (ActionToDo :type ActionsEnum%20Enum :default "NewEnumerator0"))
  (bind _gpt_behaviourtree (Variables|Default|GetGPT_BehaviourTree))
  (bind _capsulecomponent (Variables|Default|GetCapsuleComponent))
  (bind _returnvalue (Transformation|GetWorldLocation _capsulecomponent))
  (bind _stats (Variables|/Game/GPT_Code/Blueprints/GPT_BehaviourTree.GPT_BehaviourTree_C|GetStats _gpt_behaviourtree))
  (Development|PrintString (Utilities|String|EnumtoString ActionToDo))
  (switch Utilities|FlowControl|Switch|SwitchonActionsEnum ActionToDo
    (:NewEnumerator0
      (AI|Navigation|SimpleMovetoLocation (Pawn|GetController) (.RandomLocation (AI|Navigation|GetRandomReachablePointinRadius (Transformation|GetActorLocation) 6e+02 0 "/Script/AIModule.NavFilter_AIControllerDefault"))))
    (:NewEnumerator2
      (bind _keys (Utilities|Map|Keys _stats :!label _label))
      (Utilities|Map|Add _stats (Utilities|Array|Get(acopy) _keys (Utilities|Select :Index ActionToDo :NewEnumerator0 0 :NewEnumerator1 0 :NewEnumerator2 1 :NewEnumerator3 2 :NewEnumerator4 0 :NewEnumerator5 0 :NewEnumerator6 0)) (Math|Float|Clamp(Float) (+ (.Value (Utilities|Map|Find _stats (Utilities|Array|Get(acopy) _keys (Utilities|Select :Index ActionToDo :NewEnumerator0 0 :NewEnumerator1 0 :NewEnumerator2 1 :NewEnumerator3 2 :NewEnumerator4 0 :NewEnumerator5 0 :NewEnumerator6 0)))) 0.5))))
    (:NewEnumerator3
      (goto _label))
    (:NewEnumerator4
      (Niagara|SpawnSystematLocation "/Game/GPT_Code/Blueprints/AttackEffect.AttackEffect" _returnvalue (Transformation|GetWorldRotation _capsulecomponent)))
    (:NewEnumerator5
      (Niagara|SpawnSystematLocation "/Game/GPT_Code/Blueprints/VictoryEffect.VictoryEffect" _returnvalue))
    (:NewEnumerator6
      (if (Variables|Default|GetPlayerInVisual)
        (AI|Navigation|SimpleMovetoLocation (Pawn|GetController) (Transformation|GetActorLocation (Game|Player|GetPlayerPawn 0)))))))

(fn ConstructionScript
  (|CallParentFunction)
  (Rendering|SetVisibility (Variables|Default|GetViewBox) (Variables|GPT|GetBehaviourTreeActivated) false))