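; Actor component that drives its owner's behavior through GPT, requesting new actions every 15 seconds once activated.
; Each request adds starving or thirst warnings from Stats, then sends objective, surroundings, inventory and possible actions to the GameMode's GPT_Request_Component.
; It scans the response text for action enum names and passes each match to the owner via ActionMessage, printing errors otherwise.
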(event Custom|ComponentActivated
  (CallFunction|RequestAction :!label _label)
  (Utilities|FlowControl|Delay 15.0)
  (goto _label))

(event EventBeginPlay)

(event EventTick
  (params (DeltaSeconds :type Float%20%28single-precision%29)))

(fn RequestAction
  (bind _returnvalue (Game|GetGameMode))
  (bind _returnvalue_2 (Actor|GetComponentbyClass _returnvalue "/Game/GPT_Code/Blueprints/GPT_Request_Component.GPT_Request_Component_C"))
  (Utilities|IsValid _returnvalue_2
    (:Is%20Valid
      (CallFunction|CalculateNeeds)
      (bind (_response _valid) (Default|RequestResponse _returnvalue_2 (Utilities|String|Append (Variables|Default|GetObjective) " 
" (CallFunction|SurroundingInfotoText (Variables|Default|GetSurroundingInfo)) " 
" (CallFunction|InventorytoText (Variables|Default|GetInventoryInfo)) " 
" (CallFunction|PossibleAction))))
      (if _valid
        (Development|PrintString _response)
        (bind _actions (CallFunction|StringActionsReponseConverter _response))
        (for _array_element _actions
          (Class|BehaviourTreeInterface|Action(Message) (Components|GetOwner) _array_element))
        (return)
        (else
          (Development|PrintString "Response error" true true "(R=1.000000,G=0.000000,B=0.099000,A=1.000000)"))))
    (:Is%20Not%20Valid
      (Development|PrintString "ADD THE GPT REQUEST COMPONENT IN THE GAME MODE" true true "(R=1.000000,G=0.000000,B=0.000000,A=1.000000)"))))

(fn StringActionsReponseConverter
  (params (Actions%20String :type String))
  (bind _enumvalue (|ForEachActionsEnum)
    (:LoopBody
      (if (!= (Utilities|String|FindSubstring Actions%20String (Utilities|String|EnumtoString _enumvalue)) -1)
        (Utilities|Array|Add (LocalVariables|GetTempActions) _enumvalue)))
    (:then
      (return (LocalVariables|GetTempActions)))))

(fn CalculateNeeds
  (Utilities|Array|SetArrayElem (Variables|Default|GetSurroundingInfo) 2 (select (> (.Value (Utilities|Map|Find (Variables|Default|GetStats) "Food")) 0.1) (Utilities|String|MakeLiteralString) (Utilities|String|MakeLiteralString "You are starving")) true)
  (Utilities|Array|SetArrayElem (Variables|Default|GetSurroundingInfo) 3 (select (> (.Value (Utilities|Map|Find (Variables|Default|GetStats) "Water")) 0.1) (Utilities|String|MakeLiteralString) (Utilities|String|MakeLiteralString "You are dying of thirst")) true)
  (return))